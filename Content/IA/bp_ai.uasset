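; AI character Blueprint for an enemy that chases the player, printing "Game Over !" when it reaches its target.
; PawnSensing sight of the player, or a heard noise with near-zero volume, raises walk speed and starts AIMoveTo toward that pawn or instigator.
; A Ronde event patrols random reachable points, re-calling itself on success or failure; nothing here starts it or calls the Walk speed reset.
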(event OnSeePawn(PawnSensing)
  (params (Pawn :type Pawn%20Object%20Reference))
  ;[1 1 1] Vue
  (if (== Pawn (Game|GetPlayerCharacter 0))
    (CallFunction|Run)
    (AI|AIMoveTo self "0, 0, 0" Pawn 5.0 false
      (:OnSuccess
        (Development|PrintString "Game Over ! ")))))

(event OnHearNoise(PawnSensing)
  (params (Instigator :type Pawn%20Object%20Reference) (Location :type Vector%20%28by%20ref%29 :default "0, 0, 0") (Volume :type Float%20%28single-precision%29))
  (if (Math|Float|NearlyEqual(Float) Volume 0.0 0.01)
    (CallFunction|Run)
    (AI|AIMoveTo self "0, 0, 0" Instigator 5.0 false
      (:OnSuccess
        (Development|PrintString "Game Over ! ")))))

(event Custom|Ronde
  ;[1 1 1] Ronde
  (AI|AIMoveTo self (.RandomLocation (AI|Navigation|GetRandomReachablePointinRadius (Transformation|GetActorLocation) 5e+03 0 0)) 0 5.0 false
    (:OnSuccess
      _)
    (:OnFail
      _))
  (CallFunction|Ronde))

(event EventBeginPlay)

(event Collision|EventActorBeginOverlap
  (params (OtherActor :type Actor%20Object%20Reference)))

(event EventTick
  (params (DeltaSeconds :type Float%20%28single-precision%29)))

(fn ConstructionScript)

(fn Run
  (Variables|/Script/Engine.CharacterMovementComponent|SetMaxWalkSpeed (Variables|Character|GetCharacterMovement) 4e+02))

(fn Walk
  (Variables|/Script/Engine.CharacterMovementComponent|SetMaxWalkSpeed (Variables|Character|GetCharacterMovement) 178.0))